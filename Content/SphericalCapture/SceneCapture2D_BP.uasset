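; Scene capture actor Blueprint that saves a one-shot render of the scene to a timestamped HDR file.
; SaveHDR briefly activates the capture component, captures once, deactivates it, then exports its render target to a relative parent directory.
; NowString builds the zero-padded date-and-time suffix for the CaptureImage file name.
; The event graph and construction script are empty, so nothing in this Blueprint triggers the save.
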(event EventBeginPlay)

(event Collision|EventActorBeginOverlap
  (params (OtherActor :type Actor%20Object%20Reference)))

(event EventTick
  (params (DeltaSeconds :type Float%20%28single-precision%29)))

(fn ConstructionScript)

(fn SaveHDR
  (CallFunction|ShotsRenderTarget)
  (bind _nowstring (CallFunction|NowString))
  (Rendering|ExportRenderTarget (Variables|/Script/Engine.SceneCaptureComponent2D|GetTextureTarget (Variables|Default|GetSceneCaptureComponent2D)) "../../.." (Utilities|String|Append (Utilities|String|Append "CaptureImage_" _nowstring) ".hdr")))

(fn ShotsRenderTarget
  (bind _scenecapturecomponent2d (Variables|Default|GetSceneCaptureComponent2D))
  (Components|Activation|Activate _scenecapturecomponent2d false)
  (Rendering|SceneCapture|CaptureScene _scenecapturecomponent2d :!class /Script/Engine.SceneCaptureComponent2D)
  (Components|Activation|Deactivate _scenecapturecomponent2d))

(fn NowString
  (bind _returnvalue (Math|DateTime|Now))
  (bind (_year _month _day _hour _minute _second) (Math|DateTime|BreakDateTime _returnvalue))
  (return (Utilities|String|Append (Utilities|String|Append (Utilities|String|Append (Utilities|String|Append (Utilities|String|Append (Utilities|String|ToString(Integer) _year) (Utilities|String|Right (Utilities|String|Append "00" (Utilities|String|ToString(Integer) _month)) 2)) (Utilities|String|Right (Utilities|String|Append "00" (Utilities|String|ToString(Integer) _day)) 2)) (Utilities|String|Right (Utilities|String|Append "00" (Utilities|String|ToString(Integer) _hour)) 2)) (Utilities|String|Right (Utilities|String|Append "00" (Utilities|String|ToString(Integer) _minute)) 2)) (Utilities|String|Right (Utilities|String|Append "00" (Utilities|String|ToString(Integer) _second)) 2))))